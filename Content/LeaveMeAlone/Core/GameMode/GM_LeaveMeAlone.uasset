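; Game mode for LeaveMeAlone that runs the match countdown and shows the end-of-game menus.
; A looping one-second timer decrements GameTime and reads the player character's HealthComponent.
; If time runs out while the player is alive, it opens the time-over menu; after death, a DeadTime countdown delays the death menu.
; Either outcome clears the timer and switches the player controller to UI-only input.
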(event Custom|OnSecEvent
  (bind _health_component (Variables|Default|GetHealth%20Component))
  (bind _returnvalue (Class|LMAHealthComponent|IsDead _health_component))
  (Utilities|FlowControl|Sequence
    (:then_0
      (bind _output_get (Variables|Default|SetGameTime (- (Variables|Default|GetGameTime) 1)))
      (if (and (== _output_get 0) (not _returnvalue))
        (Utilities|Time|ClearandInvalidateTimerbyHandle (Variables|Default|GetGameTimerHandle))
        (bind _returnvalue_2 (UserInterface|CreateWidget "/Game/LeaveMeAlone/Widgets/UI/WBP_TimeOverMenu.WBP_TimeOverMenu_C"))
        (bind _output_get_2 (Variables|Default|SetEndGameMenu _returnvalue_2))
        (UserInterface|Viewport|AddtoViewport _output_get_2 0)
        (bind _aspc_leave_me_alone (Utilities|Casting|CastToPC_LeaveMeAlone (Game|GetPlayerController 0)))
        (Input|SetInputModeUIOnly _aspc_leave_me_alone _output_get_2 "DoNotLock" false)))
    (:then_1
      (if _returnvalue
        (bind _output_get_3 (Variables|Default|SetDeadTime (- (Variables|Default|GetDeadTime) 1)))
        (if (== _output_get_3 0)
          (Utilities|Time|ClearandInvalidateTimerbyHandle (Variables|Default|GetGameTimerHandle))
          (bind _returnvalue_3 (UserInterface|CreateWidget "/Game/LeaveMeAlone/Widgets/UI/WBP_DeadMenu.WBP_DeadMenu_C"))
          (bind _output_get_4 (Variables|Default|SetDeadMenu _returnvalue_3))
          (UserInterface|Viewport|AddtoViewport _output_get_4 0)
          (bind _aspc_leave_me_alone_2 (Utilities|Casting|CastToPC_LeaveMeAlone (Game|GetPlayerController 0)))
          (Input|SetInputModeUIOnly _aspc_leave_me_alone_2 _output_get_4 "DoNotLock" false))))))

(event EventBeginPlay
  (bind _returnvalue (Utilities|Time|SetTimerbyEvent (delegate Custom|OnSecEvent) 1.0 true))
  (Variables|Default|SetGameTimerHandle _returnvalue)
  (bind _asch_player (Utilities|Casting|CastToCH_Player (Game|GetPlayerCharacter 0)))
  (Variables|Default|SetHealth%20Component (Variables|/Script/LeaveMeAlone.LMADefaultCharacter|GetHealthComponent _asch_player)))

(event EventTick
  (params (DeltaSeconds :type Float%20%28single-precision%29)))

(fn ConstructionScript)